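; Unity-chan CRS character Blueprint that drives lip-sync animation and provides damage voice playback.
; A timeline started on BeginPlay samples five vowel float curves (A, I, U, E, O), scales them down by 100 and writes them to MTH_ morph targets.
; Tick moves the capsule to the hips bone so collision follows the animated body.
; DumageVoicePlayFunc forwards damage sound playback to a BP_UnityChanVoice child actor.
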(event `self.ReceiveBeginPlay`
  (bind (_direction _time) (`Timeline|RysyncTimeLien`)
    (:`Update`
      (`|ExecutionSequence`
        (:`then_0`
          ;[1 1 1] モーフターゲット：あ
          (`self.SetLipSync` "MTH_A" (`CurveFloat.GetFloatValue` (`self.Lips_A`) _time)))
        (:`then_1`
          ;[1 1 1] モーフターゲット：い
          (`self.SetLipSync` "MTH_I" (`CurveFloat.GetFloatValue` (`self.Lisp_I`) _time)))
        (:`then_2`
          ;[1 1 1] モーフターゲット：う
          (`self.SetLipSync` "MTH_U" (`CurveFloat.GetFloatValue` (`self.Lisp_U`) _time)))
        (:`then_3`
          ;[1 1 1] モーフターゲット：え
          (`self.SetLipSync` "MTH_E" (`CurveFloat.GetFloatValue` (`self.Lisp_E`) _time)))
        (:`then_4`
          ;[1 1 1] モーフターゲット：お
          (`self.SetLipSync` "MTH_O" (`CurveFloat.GetFloatValue` (`self.Lisp_O`) _time)))))))

(event `self.ReceiveTick`
  (params (DeltaSeconds :type "Float (single-precision)"))
  ;[1 1 1] Tickイベント　ボーンにコリジョンを追従
  (`SceneComponent.K2_SetWorldLocation` (`self.Capsule`) (`SceneComponent.GetSocketLocation` (`self.SkeletalMeshComponent`) "Character1_Hips") false false))

(fn `DumageVoicePlayFunc`
  ;[1 1 1] ダメージボイス再生処理
  (`/Game/Ogino/UnitychanAsset/voice/BP_UnityChanVoice.DumagePlaySound` (cast `/Game/Ogino/UnitychanAsset/voice/BP_UnityChanVoice` (`ChildActorComponent.ChildActor` (`self.BP_UnityChanVoice`)) :!pure true)))

(fn `SetLipSync`
  (params (Name :type Name) (lipTime :type "Float (double-precision)"))
  (`AnimInstance.SetMorphTarget` (`SkeletalMeshComponent.GetAnimInstance` (`self.SkeletalMeshComponent`)) Name (/ lipTime 100.0)))

(fn `UserConstructionScript`)