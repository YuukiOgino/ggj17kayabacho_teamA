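; Unity-chan voice actor that plays random idle, success and damage voice clips.
; A timeline acts as a repeating idle timer, playing a random default clip on each finish at boosted volume with no location wired.
; SucsessPlaySound and DumagePlaySound call StopDefult to restart that timer, then play a random clip from their own list at the actor's location.
; StopDefult only postpones the next idle line and does not stop audio already playing.
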(event `self.ReceiveBeginPlay`
  (`Timeline|SoundTimeLine` :!label _label
    (:`Finished`
      (`GameplayStatics.PlaySoundAtLocation` (`KismetArrayLibrary.Array_Get` (`self.DefultSoundBaseList`) (`KismetMathLibrary.RandomInteger` (`KismetArrayLibrary.Array_Length` (`self.DefultSoundBaseList`)))) (0.0 0.0 0.0) (struct) 50.0)
      (goto _label :!via `PlayFromStart`))))

(event `StopDefult`
  (goto _label :!via `PlayFromStart`))

(fn `DumagePlaySound`
  (`self.StopDefult`)
  (`GameplayStatics.PlaySoundAtLocation` (`KismetArrayLibrary.Array_Get` (`self.DumageSoundBaseList`) (`KismetMathLibrary.RandomInteger` (`KismetArrayLibrary.Array_Length` (`self.DumageSoundBaseList`)))) (`self.K2_GetActorLocation`)))

(fn `SucsessPlaySound`
  (`self.StopDefult`)
  (`GameplayStatics.PlaySoundAtLocation` (`KismetArrayLibrary.Array_Get` (`self.SucsessSoundBaseList`) (`KismetMathLibrary.RandomInteger` (`KismetArrayLibrary.Array_Length` (`self.SucsessSoundBaseList`)))) (`self.K2_GetActorLocation`)))

(fn `UserConstructionScript`)