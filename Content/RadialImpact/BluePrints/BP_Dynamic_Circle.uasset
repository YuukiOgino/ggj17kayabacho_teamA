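; Radial Impact's dynamic circle, which grows or shrinks past the static circle until player input stops it to score on the size difference.
; Each round copies the static circle's color, picks a random smaller or larger start scale and plays a timeline-driven lerp.
; Finishing untouched counts as a miss, while menu and game-over states trigger menu AI.
; It also fires color-matched explosions and drives BP_GameMode_Actor and HUD through references cached at construction.
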(event `self.ReceiveBeginPlay`
  ;[1 0.9306 0.04308] Sets up Player Camera
  (`PlayerController.SetViewTargetWithBlend` (`GameplayStatics.GetPlayerController` 0) (`self.Radial Impact Camera`) 0.0 "VTBlend_Linear" 0.0 false))

(event `self.ReceiveTick`
  (params (DeltaSeconds :type "Float (single-precision)"))
  ;[1 1 1] Get Delta Time
  (set `self.Delta Time` DeltaSeconds))

(event `Call Menu AI`
  ;[1 0.3404 0] Logic That Calls the Appropriate Menu AI depending on Which Game State
  (if (`/Game/RadialImpact/BluePrints/BP_Menu.bisOnMenu` (`self.Main Menu Reference`))
    (`KismetSystemLibrary.Delay` 0.1 :!label _label)
    (`/Game/RadialImpact/BluePrints/BP_GameMode_Actor.Menu Play AI` (`self.Game Mode Reference`))
    (elif (`/Game/RadialImpact/BluePrints/BP_GameMode_Actor.bClassicModeGameOver` (`self.Game Mode Reference`))
      (goto _label)
      (elif (`/Game/RadialImpact/BluePrints/BP_GameMode_Actor.bTimeTrialGameOver` (`self.Game Mode Reference`))
        (goto _label)
        (elif (`/Game/RadialImpact/BluePrints/BP_GameMode_Actor.bSelectingWavesOptions` (`self.Game Mode Reference`))
          (goto _label)
          (elif (`/Game/RadialImpact/BluePrints/BP_GameMode_Actor.bWavesModeGameOver` (`self.Game Mode Reference`))
            (goto _label)))))))

(event `Activate Particle`
  (bind _static_circle_color (`self.Static Circle Color`))
  (bind _returnvalue (* _static_circle_color _static_circle_color))
  ;[1 0.2095 0.1999] Activates and Spawns Explosion Particle for Perfect Ratings
  (`SceneComponent.K2_SetWorldLocation` (`self.Explosion Particle`) (`SceneComponent.K2_GetComponentLocation` (`/Game/RadialImpact/BluePrints/BP_Static_Circle.Static Circle` (`self.Static Circle Reference`))) false false)
  ;;[1 1 1] Matches Color of Circles to the Color of Particle
  (`ParticleSystemComponent.SetColorParameter` (`self.Explosion Particle`) "Particle Color" (* (* _returnvalue _returnvalue) 10.0) :!label _label_2)
  (`ActorComponent.Activate` (`self.Explosion Particle`) false)
  (if (`/Game/RadialImpact/BluePrints/BP_Menu.bIsGameMuted` (`self.Main Menu Reference`))
    (`KismetSystemLibrary.Delay` 0.2)
    (`ActorComponent.Deactivate` (`self.Explosion Particle`))
    (else
      (`AudioComponent.Play` (`self.Circle Explosion Sound`) 0.0)
      (`KismetSystemLibrary.Delay` 0.2)
      (`ActorComponent.Deactivate` (`self.Explosion Particle`)))))

(event `Finished Timeline Reset`
  ;[1 1 1] Logic for the Dynamic Circle
  (if (>= (`TimelineComponent.GetTimelineLength` (`self.Dynamic Circle Scaling Curve`)) 10.0)
    (if true
      (if (>= (`TimelineComponent.GetTimelineLength` (`self.Dynamic Circle Scaling Curve`)) 30.0)
        _
        (else
          _))
      (`KismetSystemLibrary.Delay` 0.3)
      (else
        (`KismetSystemLibrary.Delay` 0.1)))
    (else
      (`KismetSystemLibrary.Delay` 0.1)))
  (`TimelineComponent.Stop` (`self.Dynamic Circle Scaling Curve`))
  (if (not (`/Game/RadialImpact/BluePrints/BP_Menu.bisOnMenu` (`self.Main Menu Reference`)))
    (`/Game/RadialImpact/BluePrints/BP_GameMode_Actor.Show Missed Feedback` (`self.Game Mode Reference`))
    (if (`/Game/RadialImpact/BluePrints/BP_GameMode_Actor.bIsPlayingWavesMode` (`self.Game Mode Reference`))
      (`self.Add to Current Wave`))
    (`KismetSystemLibrary.Delay` 0.75 :!label _label_3)
    (`TimelineComponent.SetPlaybackPosition` (`self.Dynamic Circle Scaling Curve`) 0.0 false true)
    (if (not (`/Game/RadialImpact/BluePrints/BP_Menu.bisOnMenu` (`self.Main Menu Reference`)))
      (`/Game/RadialImpact/BluePrints/BP_Static_Circle.Change Color` (`self.Static Circle Reference`))
      (`KismetSystemLibrary.Delay` 0.5 :!label _label_4)
      (set `/Game/RadialImpact/BluePrints/BP_GameMode_Actor.bCanInput` true (`self.Game Mode Reference`)))))

(event `Activate Stopwatch Particle`
  ;[1 0.2095 0.1999] Activates and Spawns Explosion Particle for Perfect Ratings
  (`SceneComponent.K2_SetWorldLocation` (`self.Explosion Particle`) (`SceneComponent.K2_GetComponentLocation` (`/Game/RadialImpact/BluePrints/BP_HUDElements.StopWatch` (`self.HUD Elements Reference`))) false false)
  (goto _label_2))

(event `Logic for When Dynamic Circle is Clicked in Game`
  ;[1 1 1] Logic for the Dynamic Circle
  (if (`/Game/RadialImpact/BluePrints/BP_GameMode_Actor.bCanInput` (`self.Game Mode Reference`))
    (set `/Game/RadialImpact/BluePrints/BP_GameMode_Actor.bCanInput` false (`self.Game Mode Reference`))
    (set `/Game/RadialImpact/BluePrints/BP_GameMode_Actor.Number of Rounds for Classic Mode` (+ (`/Game/RadialImpact/BluePrints/BP_GameMode_Actor.Number of Rounds for Classic Mode` (`self.Game Mode Reference`)) 1) (`self.Game Mode Reference`))
    (`TimelineComponent.Stop` (`self.Dynamic Circle Scaling Curve`))
    (`self.Compare Size`)
    (goto _label_3)))

(event `Update Dynamic Color`
  ;[1 1 1] Logic for the Dynamic Circle
  ;;[1 1 1] Matches the Color of the Dynamic Circle with the Color of the Static Circle
  (if (not (`self.bIsGamePaused`)) :!label _label_5
    (bind _returnvalue (`MaterialInstanceDynamic.K2_GetVectorParameterValue` (`/Game/RadialImpact/BluePrints/BP_Static_Circle.Static Circle MI` (`self.Static Circle Reference`)) "Static Circle Color"))
    (set `self.Static Circle Color` _returnvalue)
    (`MaterialInstanceDynamic.SetVectorParameterValue` (`self.Dynamic Circle MI`) "Dynamic Circle Color" (`self.Static Circle Color`))
    (`self.Set Size of Dynamic Circle`)))

(event `Compare Size`
  (bind _x (.x (`SceneComponent.K2_GetComponentScale` (`self.Dynamic Circle`))))
  (bind _x_2 (.x (`SceneComponent.K2_GetComponentScale` (`/Game/RadialImpact/BluePrints/BP_Static_Circle.Static Circle` (`self.Static Circle Reference`)))))
  ;[0.4268 1 0.02583] Gets Comparable Sizes of Dynamic/Static Circle and Finds Which One is Larger When Clicked
  (if (not (`/Game/RadialImpact/BluePrints/BP_Menu.bIsGamePaused?` (`self.Main Menu Reference`)))
    ;;[1 1 1] Compares the Size of the Two Circles
    (if (> _x _x_2)
      ;;[1 1 1] Applies the Appropriate Scoring Based on Which Circle is Bigger
      (set `self.Dynamic - Static` (`KismetMathLibrary.Abs` (- _x_2 _x)))
      (`/Game/RadialImpact/BluePrints/BP_GameMode_Actor.Apply Score Dynamic - Static` (`self.Game Mode Reference`))
      (else
        (set `self.Static - Dynamic` (`KismetMathLibrary.Abs` (- _x _x_2)))
        (`/Game/RadialImpact/BluePrints/BP_GameMode_Actor.Apply Score Static - Dynamic` (`self.Game Mode Reference`))))))

(event `Begin Playing Classic Mode`
  ;[1 1 1] Logic for the Dynamic Circle
  (set `/Game/RadialImpact/BluePrints/BP_Menu.bisOnMenu` false (`self.Main Menu Reference`))
  (`|ExecutionSequence`
    (:`then_0`
      (if (`TimelineComponent.IsPlaying` (`self.Dynamic Circle Scaling Curve`))
        (`TimelineComponent.Stop` (`self.Dynamic Circle Scaling Curve`))
        (goto _label_3)
        (else
          (goto _label_4))))
    (:`then_1`
      (set `/Game/RadialImpact/BluePrints/BP_GameMode_Actor.bCanInput` false (`self.Game Mode Reference`))
      (`KismetSystemLibrary.Delay` 1.0)
      (set `/Game/RadialImpact/BluePrints/BP_GameMode_Actor.bIsClassicModePlaying` true (`self.Game Mode Reference`))
      (`/Game/RadialImpact/BluePrints/BP_Menu.Set Game HUD` (`self.Main Menu Reference`)))))

(event `Set Dynamic Circle`
  ;[1 1 1] Logic for the Dynamic Circle
  ;;[1 1 1] Matches the Color of the Dynamic Circle with the Color of the Static Circle
  (goto _label_5))

(event `Reset for Play Rate on Waves and Classic mode`
  ;[1 1 1] Logic for the Dynamic Circle
  ;;[1 1 1] Calls Menu AI and Resets Play Rate of the Dynamic Circle Animation
  (`/Game/RadialImpact/BluePrints/BP_GameMode_Actor.Set Animation Play Rate Classic Mode` (`self.Game Mode Reference`))
  (`/Game/RadialImpact/BluePrints/BP_GameMode_Actor.Set Animation Play Rate Waves Mode` (`self.Game Mode Reference`))
  (`TimelineComponent.PlayFromStart` (`self.Dynamic Circle Scaling Curve`) :!label _label_6))

(event `Call Menu AI and Reset Playrates`
  ;[1 1 1] Logic for the Dynamic Circle
  ;;[1 1 1] Calls Menu AI and Resets Play Rate of the Dynamic Circle Animation
  (`self.Call Menu AI`)
  (`TimelineComponent.SetPlayRate` (`self.Dynamic Circle Scaling Curve`) 1.0)
  (goto _label_6))

(event `Reset Play Rate and Time Length`
  (bind _dynamic_circle_scaling_curve (`self.Dynamic Circle Scaling Curve`))
  ;[0.3746 1 0.05634] Slows Down the Play Rate of the Dynamic Circle and Sets Current Play Rates into Variables
  ;;[1 1 1] Sets Variables of Play Rate and Time Length Before Slow Down
  (`TimelineComponent.SetPlayRate` _dynamic_circle_scaling_curve (`self.Current Play Rate of Dynamic Circle`))
  (`TimelineComponent.SetTimelineLength` _dynamic_circle_scaling_curve (`self.Current Time Length of Dynamic Circle`)))

(event `Update Dynamic Circle Size`
  ;[1 1 1] Logic for the Dynamic Circle
  ;;[1 1 1] Calls the Appropriate MENU AI based on Game State
  (if (`/Game/RadialImpact/BluePrints/BP_GameMode_Actor.bTimeTrialGameOver` (`self.Game Mode Reference`))
    (`self.Call Menu AI and Reset Playrates`)
    (elif (`/Game/RadialImpact/BluePrints/BP_GameMode_Actor.bClassicModeGameOver` (`self.Game Mode Reference`))
      (`self.Call Menu AI and Reset Playrates`)
      (elif (`/Game/RadialImpact/BluePrints/BP_GameMode_Actor.bWavesModeGameOver` (`self.Game Mode Reference`))
        (`self.Call Menu AI and Reset Playrates`)
        (elif (`/Game/RadialImpact/BluePrints/BP_GameMode_Actor.bSelectingWavesOptions` (`self.Game Mode Reference`))
          (`self.Call Menu AI and Reset Playrates`)
          (elif (`/Game/RadialImpact/BluePrints/BP_Menu.bIsGamePaused?` (`self.Main Menu Reference`))
            _
            (elif (`/Game/RadialImpact/BluePrints/BP_Menu.bisOnMenu` (`self.Main Menu Reference`))
              (`self.Call Menu AI and Reset Playrates`)
              (else
                (`self.Reset for Play Rate on Waves and Classic mode`)))))))))

(event `self.Dynamic Circle.OnClicked`
  (params (TouchedComponent :type "PrimitiveComponent Object Reference") (ButtonPressed :type "Key Structure" :default "AnyKey"))
  ;[1 1 1] Logic for the Dynamic Circle
  ;;[1 1 1] Logic for Clicking on Dynamic Circle during a Game Mode
  (if (`/Game/RadialImpact/BluePrints/BP_Menu.bisOnMenu` (`self.Main Menu Reference`)) :!label _label_7
    (`self.Begin Playing Classic Mode`)
    (elif (`/Game/RadialImpact/BluePrints/BP_GameMode_Actor.bIsClassicModePlaying` (`self.Game Mode Reference`))
      (`self.Logic for When Dynamic Circle is Clicked in Game`)
      (elif (`/Game/RadialImpact/BluePrints/BP_GameMode_Actor.bIsPlayingTimeTrial` (`self.Game Mode Reference`))
        (`self.Logic for When Dynamic Circle is Clicked in Game`)
        (elif (`/Game/RadialImpact/BluePrints/BP_GameMode_Actor.bIsPlayingWavesMode` (`self.Game Mode Reference`))
          (`self.Logic for When Dynamic Circle is Clicked in Game`))))))

(event `Slow Play Rate`
  (bind _dynamic_circle_scaling_curve (`self.Dynamic Circle Scaling Curve`))
  ;[0.3746 1 0.05634] Slows Down the Play Rate of the Dynamic Circle and Sets Current Play Rates into Variables
  ;;[1 1 1] Slows Down Play Rate and Timeline Length
  (`TimelineComponent.SetPlayRate` _dynamic_circle_scaling_curve 0.5)
  (`TimelineComponent.SetTimelineLength` _dynamic_circle_scaling_curve 1.5))

(event `SpaceBar`
  ;[1 1 1] Logic for the Dynamic Circle
  ;;[1 1 1] Logic for Clicking on Dynamic Circle during a Game Mode
  (goto _label_7))

(event `Static Circle Clicked`
  ;[1 1 1] Logic for the Dynamic Circle
  (goto _label_7))

(event `self.ReceiveActorOnInputTouchBegin`
  (params (FingerIndex :type "ETouchIndex Enum" :default "Touch1"))
  ;[1 1 1] Logic for the Dynamic Circle
  ;;[1 1 1] Logic for Clicking on Dynamic Circle during a Game Mode
  (goto _label_7))

(event `Static Circle Touched`
  ;[1 1 1] Logic for the Dynamic Circle
  (goto _label_7))

(event `self.Dynamic Circle.OnInputTouchBegin`
  (params (FingerIndex :type "ETouchIndex Enum" :default "Touch1") (TouchedComponent :type "PrimitiveComponent Object Reference"))
  ;[1 1 1] Logic for the Dynamic Circle
  ;;[1 1 1] Logic for Clicking on Dynamic Circle during a Game Mode
  (goto _label_7))

(event `Small Dynamic Circle`
  (bind _returnvalue (`SceneComponent.K2_GetComponentScale` (`/Game/RadialImpact/BluePrints/BP_Static_Circle.Static Circle` (`self.Static Circle Reference`))))
  (bind _returnvalue_2 (/ _returnvalue (`KismetMathLibrary.RandomFloatInRange` 2.0 3.5)))
  ;[0.2074 1 0] Sets the Size of the Dynamic Circle - Either Setting it Smaller or Larger Than the Static Circle
  ;;[1 1 1] Sets Size of Dynamic Circle Smaller Than the Static Circle
  (if (`/Game/RadialImpact/BluePrints/BP_Menu.bIsGamePaused?` (`self.Main Menu Reference`)) :!label _label_8
    _
    (elif (== _returnvalue_2 _returnvalue :`ErrorTolerance` 0.0)
      (goto _label_8)
      (else
        (`SceneComponent.SetRelativeScale3D` (`self.Dynamic Circle`) _returnvalue_2)))))

(event `Print Bools`
  ;[1 1 1] Print Bool Variables
  (`KismetSystemLibrary.PrintString` (`KismetStringLibrary.Concat_StrStr` "Is Classic Mode Playing: " (`KismetStringLibrary.Conv_BoolToString` (`/Game/RadialImpact/BluePrints/BP_GameMode_Actor.bIsClassicModePlaying` (`self.Game Mode Reference`)))))
  (`KismetSystemLibrary.PrintString` (`KismetStringLibrary.Concat_StrStr` "Is Time Trial Mode Playing: " (`KismetStringLibrary.Conv_BoolToString` (`/Game/RadialImpact/BluePrints/BP_GameMode_Actor.bIsPlayingTimeTrial` (`self.Game Mode Reference`)))))
  (`KismetSystemLibrary.PrintString` (`KismetStringLibrary.Concat_StrStr` "Is Waves Mode Playing: " (`KismetStringLibrary.Conv_BoolToString` (`/Game/RadialImpact/BluePrints/BP_GameMode_Actor.bIsPlayingWavesMode` (`self.Game Mode Reference`))))))

(event `Large Dynamic Circle`
  (bind _returnvalue (`SceneComponent.K2_GetComponentScale` (`/Game/RadialImpact/BluePrints/BP_Static_Circle.Static Circle` (`self.Static Circle Reference`))))
  (bind _returnvalue_2 (* _returnvalue (`KismetMathLibrary.RandomFloatInRange` 2.0 3.5)))
  ;[0.2074 1 0] Sets the Size of the Dynamic Circle - Either Setting it Smaller or Larger Than the Static Circle
  ;;[1 1 1] Sets Size of Dynamic Circle Larger Than Static
  (if (`/Game/RadialImpact/BluePrints/BP_Menu.bIsGamePaused?` (`self.Main Menu Reference`)) :!label _label_9
    _
    (elif (== _returnvalue _returnvalue_2 :`ErrorTolerance` 0.0)
      (goto _label_9)
      (else
        (`SceneComponent.SetRelativeScale3D` (`self.Dynamic Circle`) _returnvalue_2)))))

(event `Set Size of Dynamic Circle`
  ;[0.1366 1 0] Updates the Comparable Size of the Dynamic Circle to the Static Circle
  (if (not (`/Game/RadialImpact/BluePrints/BP_Menu.bIsGamePaused?` (`self.Main Menu Reference`)))
    (if (== (`KismetMathLibrary.RandomIntegerInRange` 1 2) 1)
      (`self.Small Dynamic Circle`)
      (set `self.bIsDynamicCircleSmall` true)
      (else
        (`self.Large Dynamic Circle`)
        (set `self.bIsDynamicCircleSmall` false)))
    (`KismetSystemLibrary.Delay` 0.5)
    (`self.Update Dynamic Circle Size`)))

(event `Add to Current Wave`
  ;[0.1821 1 0.1143] Adds to the Current Number of Waves for Wave Mode
  (set `self.Current Wave` (+ (`self.Current Wave`) 1))
  (if (> (`self.Current Wave`) 9)
    (`TextRenderComponent.SetText` (`/Game/RadialImpact/BluePrints/BP_HUDElements.Current Wave Number` (`self.HUD Elements Reference`)) (`KismetStringLibrary.Conv_IntToString` (`self.Current Wave`)))
    (`/Game/RadialImpact/BluePrints/BP_GameMode_Actor.Check if Waves Mode is Over` (`self.Game Mode Reference`))
    (else
      (`TextRenderComponent.SetText` (`/Game/RadialImpact/BluePrints/BP_HUDElements.Current Wave Number` (`self.HUD Elements Reference`)) (`KismetStringLibrary.Concat_StrStr` "0" (`KismetStringLibrary.Conv_IntToString` (`self.Current Wave`))))
      (`/Game/RadialImpact/BluePrints/BP_GameMode_Actor.Check if Waves Mode is Over` (`self.Game Mode Reference`)))))

(fn `UserConstructionScript`
  (locals (NewLocalVar_0 :type Boolean) (NewLocalVar_1 :type Boolean))
  (bind _outactors (`GameplayStatics.GetAllActorsOfClass` "/Game/RadialImpact/BluePrints/BP_Static_Circle.BP_Static_Circle_C"))
  (bind _asbp_static_circle (cast `/Game/RadialImpact/BluePrints/BP_Static_Circle` (`KismetArrayLibrary.Array_Get` _outactors)))
  (set `self.Static Circle Reference` _asbp_static_circle)
  (bind _returnvalue (`PrimitiveComponent.CreateDynamicMaterialInstance` (`self.Dynamic Circle`) 0 null))
  (set `self.Dynamic Circle MI` _returnvalue)
  (`MaterialInstanceDynamic.SetScalarParameterValue` (`self.Dynamic Circle MI`) "Dynamic Circle Intensity" 3.0)
  (bind _outactors_2 (`GameplayStatics.GetAllActorsOfClass` "/Game/RadialImpact/BluePrints/BP_PlayerFeedBack_Text.BP_PlayerFeedBack_Text_C"))
  (bind _asbp_player_feed_back_text (cast `/Game/RadialImpact/BluePrints/BP_PlayerFeedBack_Text` (`KismetArrayLibrary.Array_Get` _outactors_2)))
  (set `self.Feedback Text Reference` _asbp_player_feed_back_text)
  (bind _outactors_3 (`GameplayStatics.GetAllActorsOfClass` "/Game/RadialImpact/BluePrints/BP_RadialImpact_Camera.BP_RadialImpact_Camera_C"))
  (bind _asbp_radial_impact_camera (cast `/Game/RadialImpact/BluePrints/BP_RadialImpact_Camera` (`KismetArrayLibrary.Array_Get` _outactors_3)))
  (set `self.Radial Impact Camera` _asbp_radial_impact_camera)
  (bind _outactors_4 (`GameplayStatics.GetAllActorsOfClass` "/Game/RadialImpact/BluePrints/BP_ScoreText.BP_ScoreText_C"))
  (bind _asbp_score_text (cast `/Game/RadialImpact/BluePrints/BP_ScoreText` (`KismetArrayLibrary.Array_Get` _outactors_4)))
  (set `self.Score Text Reference` _asbp_score_text)
  (bind _outactors_5 (`GameplayStatics.GetAllActorsOfClass` "/Game/RadialImpact/BluePrints/BP_HUDElements.BP_HUDElements_C"))
  (bind _asbp_hudelements (cast `/Game/RadialImpact/BluePrints/BP_HUDElements` (`KismetArrayLibrary.Array_Get` _outactors_5)))
  (set `self.HUD Elements Reference` _asbp_hudelements)
  (bind _outactors_6 (`GameplayStatics.GetAllActorsOfClass` "/Game/RadialImpact/BluePrints/BP_Menu.BP_Menu_C"))
  (bind _asbp_menu (cast `/Game/RadialImpact/BluePrints/BP_Menu` (`KismetArrayLibrary.Array_Get` _outactors_6)))
  (set `self.Main Menu Reference` _asbp_menu)
  (bind _outactors_7 (`GameplayStatics.GetAllActorsOfClass` "/Game/RadialImpact/BluePrints/BP_GameMode_Actor.BP_GameMode_Actor_C"))
  (bind _asbp_game_mode_actor (cast `/Game/RadialImpact/BluePrints/BP_GameMode_Actor` (`KismetArrayLibrary.Array_Get` _outactors_7)))
  (set `self.Game Mode Reference` _asbp_game_mode_actor))