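; BP_Music is the game's music player, playing nine songs in sequence from BeginPlay using hardcoded delays, with no loop back after the last.
; Its construction script caches the first BP_Menu, whose IsGameMuted flag is checked before each song after the first.
; AudioisPressed silences the currently playing song when muted, or restores the volume multiplier on all songs when unmuted.
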(event `self.ReceiveBeginPlay`
  ;[1 1 1] Song Loop Playlist
  (`AudioComponent.Play` (`self.Song 01`) 0.0)
  (`KismetSystemLibrary.Delay` 289.0)
  (if (`/Game/RadialImpact/BluePrints/BP_Menu.bIsGameMuted` (`self.Main Menu Reference`))
    (`AudioComponent.SetVolumeMultiplier` (`self.Song 02`) 0.0))
  (`AudioComponent.Play` (`self.Song 02`) 0.0)
  (`KismetSystemLibrary.Delay` 208.0)
  (if (`/Game/RadialImpact/BluePrints/BP_Menu.bIsGameMuted` (`self.Main Menu Reference`))
    (`AudioComponent.SetVolumeMultiplier` (`self.Song 03`) 0.0))
  (`AudioComponent.Play` (`self.Song 03`) 0.0)
  (`KismetSystemLibrary.Delay` 291.0)
  (if (`/Game/RadialImpact/BluePrints/BP_Menu.bIsGameMuted` (`self.Main Menu Reference`))
    (`AudioComponent.SetVolumeMultiplier` (`self.Song 04`) 0.0))
  (`AudioComponent.Play` (`self.Song 04`) 0.0)
  (`KismetSystemLibrary.Delay` 261.0)
  (if (`/Game/RadialImpact/BluePrints/BP_Menu.bIsGameMuted` (`self.Main Menu Reference`))
    (`AudioComponent.SetVolumeMultiplier` (`self.Song 05`) 0.0))
  (`AudioComponent.Play` (`self.Song 05`) 0.0)
  (`KismetSystemLibrary.Delay` 328.0)
  (if (`/Game/RadialImpact/BluePrints/BP_Menu.bIsGameMuted` (`self.Main Menu Reference`))
    (`AudioComponent.SetVolumeMultiplier` (`self.Song 06`) 0.0))
  (`AudioComponent.Play` (`self.Song 06`) 0.0)
  (`KismetSystemLibrary.Delay` 298.0)
  (if (`/Game/RadialImpact/BluePrints/BP_Menu.bIsGameMuted` (`self.Main Menu Reference`))
    (`AudioComponent.SetVolumeMultiplier` (`self.Song 07`) 0.0))
  (`AudioComponent.Play` (`self.Song 07`) 0.0)
  (`KismetSystemLibrary.Delay` 338.0)
  (if (`/Game/RadialImpact/BluePrints/BP_Menu.bIsGameMuted` (`self.Main Menu Reference`))
    (`AudioComponent.SetVolumeMultiplier` (`self.Song 08`) 0.0))
  (`AudioComponent.Play` (`self.Song 08`) 0.0)
  (`KismetSystemLibrary.Delay` 554.0)
  (if (`/Game/RadialImpact/BluePrints/BP_Menu.bIsGameMuted` (`self.Main Menu Reference`))
    (`AudioComponent.SetVolumeMultiplier` (`self.Song 09`) 0.0))
  (`AudioComponent.Play` (`self.Song 09`) 0.0)
  (`KismetSystemLibrary.Delay` 242.0))

(event `Audio is Pressed`
  ;[1 1 1] Check Which Song is Playing and Mute/Umute
  (if (`/Game/RadialImpact/BluePrints/BP_Menu.bIsGameMuted` (`self.Main Menu Reference`))
    (if (`AudioComponent.IsPlaying` (`self.Song 01`))
      (`AudioComponent.SetVolumeMultiplier` (`self.Song 01`) 0.0)
      (elif (`AudioComponent.IsPlaying` (`self.Song 02`))
        (`AudioComponent.SetVolumeMultiplier` (`self.Song 02`) 0.0)
        (elif (`AudioComponent.IsPlaying` (`self.Song 03`))
          (`AudioComponent.SetVolumeMultiplier` (`self.Song 03`) 0.0)
          (elif (`AudioComponent.IsPlaying` (`self.Song 04`))
            (`AudioComponent.SetVolumeMultiplier` (`self.Song 04`) 0.0)
            (elif (`AudioComponent.IsPlaying` (`self.Song 05`))
              (`AudioComponent.SetVolumeMultiplier` (`self.Song 05`) 0.0)
              (elif (`AudioComponent.IsPlaying` (`self.Song 06`))
                (`AudioComponent.SetVolumeMultiplier` (`self.Song 06`) 0.0)
                (elif (`AudioComponent.IsPlaying` (`self.Song 07`))
                  (`AudioComponent.SetVolumeMultiplier` (`self.Song 07`) 0.0)
                  (elif (`AudioComponent.IsPlaying` (`self.Song 08`))
                    (`AudioComponent.SetVolumeMultiplier` (`self.Song 08`) 0.0)
                    (elif (`AudioComponent.IsPlaying` (`self.Song 09`))
                      (`AudioComponent.SetVolumeMultiplier` (`self.Song 09`) 0.0))))))))))
    (else
      (`AudioComponent.SetVolumeMultiplier` (`self.Song 02`) 1.5)
      (`AudioComponent.SetVolumeMultiplier` (`self.Song 01`) 1.5)
      (`AudioComponent.SetVolumeMultiplier` (`self.Song 03`) 1.5)
      (`AudioComponent.SetVolumeMultiplier` (`self.Song 04`) 1.5)
      (`AudioComponent.SetVolumeMultiplier` (`self.Song 05`) 1.5)
      (`AudioComponent.SetVolumeMultiplier` (`self.Song 06`) 1.5)
      (`AudioComponent.SetVolumeMultiplier` (`self.Song 07`) 1.5)
      (`AudioComponent.SetVolumeMultiplier` (`self.Song 08`) 1.5)
      (`AudioComponent.SetVolumeMultiplier` (`self.Song 09`) 1.5))))

(fn `UserConstructionScript`
  (bind _outactors (`GameplayStatics.GetAllActorsOfClass` "/Game/RadialImpact/BluePrints/BP_Menu.BP_Menu_C"))
  (bind _asbp_menu (cast `/Game/RadialImpact/BluePrints/BP_Menu` (`KismetArrayLibrary.Array_Get` _outactors)))
  (set `self.Main Menu Reference` _asbp_menu))