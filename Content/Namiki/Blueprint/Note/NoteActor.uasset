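; VR rhythm-game note actor that spins along its owner spline and destroys itself at the end.
; On spawn, a random MultiGate occasionally gives it a holographic material.
; Motion controller overlaps play sound and random particle emitters, with only one gate output raising GameInstance Score and Combo; BP_MotionController overlap also destroys it.
; Hitting BP_UnityChanCRS triggers her damage voice and an explosion.
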(event `self.ReceiveBeginPlay`
  (bind _staticmesh (`self.StaticMesh`))
  ;[1 1 1] たまにホログラフィックのマテリアルが当たったノーツを出す
  (`|MultiGate` true true
    (:`Out 3`
      (`PrimitiveComponent.SetMaterial` _staticmesh 0 "/Game/Geeky/M_Tut_HoloB_3.M_Tut_HoloB_3"))
    (:`Out 6`
      (`PrimitiveComponent.SetMaterial` _staticmesh 0 "/Game/Geeky/M_Tut_HoloB_2.M_Tut_HoloB_2"))
    (:`Out 9`
      (`PrimitiveComponent.SetMaterial` _staticmesh 0 "/Game/Geeky/M_Tut_HoloB_1.M_Tut_HoloB_1"))))

(event `self.ReceiveActorBeginOverlap`
  (params (OtherActor :type "Actor Object Reference"))
  (bind _asbp_motion_controller (cast `/Game/VirtualRealityBP/Blueprints/BP_MotionController` OtherActor))
  ;[0.3473 0.1797 1] 消滅時にパーティクルを出す
  (`|MultiGate` true true
    (:`Out 0`
      (bind _returnvalue (`self.K2_GetActorLocation` _asbp_motion_controller))
      (`GameplayStatics.SpawnEmitterAtLocation` null _returnvalue))
    (:`Out 1`
      (`GameplayStatics.SpawnEmitterAtLocation` null _returnvalue))
    (:`Out 2`
      (`GameplayStatics.SpawnEmitterAtLocation` null _returnvalue (struct))))
  (`self.K2_DestroyActor`))

(event `self.ReceiveTick`
  (params (DeltaSeconds :type "Float (single-precision)"))
  (`self.K2_AddActorLocalRotation` (`KismetMathLibrary.MakeRotator` 0.0 (* DeltaSeconds 100.0)))
  (bind _output_get (set `self.MoveDistance` (+ (* DeltaSeconds (`self.Speed`)) (`self.MoveDistance`))))
  (bind _location (`self.GetCurrentLocation` (`self.OwnerSplineComponent`) _output_get))
  (`self.K2_SetActorLocation` _location)
  (bind _isarrived (`self.IsArrived` (`self.OwnerSplineComponent`) (`self.MoveDistance`)))
  (if _isarrived
    (`self.K2_DestroyActor`)))

(event `self.StaticMesh.OnComponentBeginOverlap`
  (params (OverlappedComponent :type "PrimitiveComponent Object Reference") (OtherActor :type "Actor Object Reference") (OtherComp :type "PrimitiveComponent Object Reference") (OtherBodyIndex :type Integer) (bFromSweep :type Boolean) (SweepResult :type "HitResult Structure (by ref)"))
  (bind _asbp_motion_controller (cast `/Game/VirtualRealityBP/Blueprints/BP_MotionController` OtherActor)
    (:`then`
      ;[0.202 1 0.2814] ノーツに触ったら音を出す
      (`GameplayStatics.PlaySoundAtLocation` "/Game/Geeky/se/Hi-tech_Digital_Item_2.Hi-tech_Digital_Item_2" (`SceneComponent.K2_GetComponentLocation` (`self.StaticMesh`)) (struct) 2.0 1.0 0.0 "/Game/Geeky/GGJSoundAttenuation.GGJSoundAttenuation")
      ;[0.3473 0.1797 1] 消滅時にパーティクルを出す
      (`|MultiGate` true true
        (:`Out 0`
          (bind _returnvalue (`SceneComponent.K2_GetComponentLocation` (`/Game/VirtualRealityBP/Blueprints/BP_MotionController.GrabSphere` _asbp_motion_controller)))
          (`GameplayStatics.SpawnEmitterAtLocation` null _returnvalue)
          (bind _asggjgame_instans (cast `/Game/Iwamoto/GGJGameinstans` (`GameplayStatics.GetGameInstance`) :!label _label))
          (bind _score (`/Game/Iwamoto/GGJGameinstans.score` _asggjgame_instans))
          (`KismetSystemLibrary.PrintString` (`KismetStringLibrary.Conv_IntToString` _score))
          (set `/Game/Iwamoto/GGJGameinstans.score` (+ _score 1) _asggjgame_instans)
          (set `/Game/Iwamoto/GGJGameinstans.combo` (+ (`/Game/Iwamoto/GGJGameinstans.combo` _asggjgame_instans) 1) _asggjgame_instans))
        (:`Out 1`
          (`GameplayStatics.SpawnEmitterAtLocation` null _returnvalue))
        (:`Out 2`
          (`GameplayStatics.SpawnEmitterAtLocation` null _returnvalue))))
    (:`CastFailed`
      (bind _asbp_right_motion_controller (cast `/Game/VirtualRealityBP/Blueprints/BP_RightMotionController` OtherActor)
        (:`then`
          (`GameplayStatics.PlaySoundAtLocation` "/Game/Geeky/se/Hi-tech_Digital_Item_2.Hi-tech_Digital_Item_2" (`SceneComponent.K2_GetComponentLocation` (`self.StaticMesh`)) (struct) 2.0 1.0 0.0 "/Game/Geeky/GGJSoundAttenuation.GGJSoundAttenuation")
          (`|MultiGate` true true
            (:`Out 0`
              (bind _returnvalue_2 (`SceneComponent.K2_GetComponentLocation` (`/Game/VirtualRealityBP/Blueprints/BP_RightMotionController.GrabSphere` _asbp_right_motion_controller)))
              (`GameplayStatics.SpawnEmitterAtLocation` null _returnvalue_2)
              (goto _label))
            (:`Out 1`
              (`GameplayStatics.SpawnEmitterAtLocation` null _returnvalue_2))
            (:`Out 2`
              (`GameplayStatics.SpawnEmitterAtLocation` null _returnvalue_2))))
        (:`CastFailed`
          ;[1 1 1] ユニティちゃんＣＲＳの場合
          (bind _asbp_unity_chan_crs (cast `/Game/Ogino/UnitychanAsset/unitychan/BP_UnityChanCRS` OtherActor))
          (`/Game/Ogino/UnitychanAsset/unitychan/BP_UnityChanCRS.DumageVoicePlayFunc` _asbp_unity_chan_crs)
          (`GameplayStatics.SpawnEmitterAtLocation` "/Game/StarterContent/Particles/P_Explosion.P_Explosion" (`SceneComponent.K2_GetComponentLocation` (`self.DefaultSceneRoot`))))))))

(fn `GetCurrentLocation`
  (params (SplineComponent :type "SplineComponent Object Reference") (Length :type "Float (double-precision)") (IsLoop :type Boolean))
  (returns (Location :type "Vector Structure"))
  (locals (LocalLength :type "Float (double-precision)"))
  (if IsLoop
    (set `local.LocalLength` (mod Length (`SplineComponent.GetSplineLength` SplineComponent)))
    (else
      (set `local.LocalLength` Length)))
  (return (`SplineComponent.GetLocationAtDistanceAlongSpline` SplineComponent (`local.LocalLength`) "World")))

(fn `IsArrived`
  (params (SplineComponent :type "SplineComponent Object Reference") (Length :type "Float (double-precision)"))
  (returns (IsArrived :type Boolean))
  (return (>= Length (`SplineComponent.GetSplineLength` SplineComponent))))

(fn `UserConstructionScript`)